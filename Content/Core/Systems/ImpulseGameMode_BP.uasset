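; Game mode for Impulse that runs an intro camera move and start countdown in any level without "Menu" in its name.
; On BeginPlay it freezes the player and possesses a CircleInPawn spawned at a random angle on a raised circle around the player camera.
; Tick lerps that pawn toward the camera position while facing the die, then shows W_Timer for three seconds before repossessing the player and restoring input and physics.
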(event EventBeginPlay
  (bind _returnvalue (Game|GetCurrentLevelName true))
  (Variables|Default|SetCurrentLevelName _returnvalue)
  (if (not (Class|VictoryBPFunctionLibrary|HasSubstring _returnvalue "Menu" "IgnoreCase" "FromStart"))
    (CallFunction|BeginNonMenuLevel)))

(event EventTick
  (params (DeltaSeconds :type Float%20%28single-precision%29))
  (bind _timer (Variables|Default|GetTimer))
  (bind _timetillstart (Variables|Default|GetTimeTillStart))
  (bind _as_impulse_player_1_bp (Variables|Default|GetAs%20Impulse%20Player%201%20BP))
  (bind _timerwidget (Variables|Default|GetTimerWidget))
  (bind _returnvalue (- _timetillstart _timer))
  (if (not (Class|VictoryBPFunctionLibrary|HasSubstring (Variables|Default|GetCurrentLevelName) "Menu" "IgnoreCase" "FromStart"))
    (if (not (< (Variables|Default|GetTimer) (- (Variables|Default|GetTimeTillStart) 3.0)))
      (if (not (Variables|Default|GetStarted))
        (Class|VictoryBPFunctionLibrary|VictoryFloatPlusEquals (Variables|Default|GetTimer) DeltaSeconds)
        (Widget|SetVisibility _timerwidget "Visible")
        (Default|CountDown _timerwidget _returnvalue)
        (if (<= _returnvalue 0.0)
          (Pawn|Possess (Variables|Default|GetPlayerController) _as_impulse_player_1_bp)
          (Variables|Default|SetStarted true)
          (Input|EnableInput _as_impulse_player_1_bp (Variables|Default|GetPlayerController))
          (Physics|SetSimulatePhysics (Variables|/Game/Core/ActorsAndControllers/ImpulsePlayer1_BP.ImpulsePlayer1_BP_C|GetSphere _as_impulse_player_1_bp) true)
          (Utilities|FlowControl|Delay 2.0)
          (Widget|RemovefromParent (Variables|Default|GetTimerWidget))))
      (else
        (CallFunction|MoveCamPawn DeltaSeconds)))))

(fn ConstructionScript)

(fn MoveCamPawn
  (params (DeltaTime :type Float%20%28single-precision%29))
  (bind _playercampawn (Variables|Default|GetPlayerCamPawn))
  (bind _floatout (Class|VictoryBPFunctionLibrary|VictoryFloatPlusEquals (Variables|Default|GetTimer) DeltaTime))
  (Transformation|SetActorLocationAndRotation _playercampawn (Math|Vector|Lerp(Vector) (Variables|Default|GetSpawnedCamLocation) (Variables|Default|GetPlayerCameraLocation) (/ _floatout (- (Variables|Default|GetTimeTillStart) 3.0))) (Math|Rotator|FindLookatRotation (Transformation|GetWorldLocation (Variables|/Game/Core/ActorsAndControllers/CircleInPawn.CircleInPawn_C|GetDefaultSceneRoot _playercampawn)) (Variables|Default|GetLookatLocation)) true true))

(fn BeginNonMenuLevel
  (bind _returnvalue (UserInterface|CreateWidget "/Game/UI/Timer/w_Timer.w_Timer_C"))
  (bind _output_get (Variables|Default|SetTimerWidget _returnvalue))
  (UserInterface|Viewport|AddtoViewport _output_get 0)
  (Widget|SetVisibility _output_get "Hidden")
  (bind _asimpulse_player_1_bp (Utilities|Casting|CastToImpulsePlayer1_BP (Game|Player|GetPlayerPawn 0)))
  (Physics|SetSimulatePhysics (Variables|/Game/Core/ActorsAndControllers/ImpulsePlayer1_BP.ImpulsePlayer1_BP_C|GetSphere _asimpulse_player_1_bp) false)
  (bind _output_get_2 (Variables|Default|SetAs%20Impulse%20Player%201%20BP _asimpulse_player_1_bp))
  (Variables|Default|SetLookatLocation (Transformation|GetWorldLocation (Variables|/Game/Core/ActorsAndControllers/ImpulsePlayer1_BP.ImpulsePlayer1_BP_C|GetDie _output_get_2)))
  (Variables|Default|SetPlayerCameraRotation (Transformation|GetWorldRotation (Variables|/Game/Core/ActorsAndControllers/ImpulsePlayer1_BP.ImpulsePlayer1_BP_C|GetDie _output_get_2)))
  (bind _output_get_3 (Variables|Default|SetPlayerController (Game|GetPlayerController 0)))
  (Input|DisableInput _output_get_2 _output_get_3)
  (Variables|Default|SetPlayerCameraLocation (Transformation|GetWorldLocation (Variables|/Game/Core/ActorsAndControllers/ImpulsePlayer1_BP.ImpulsePlayer1_BP_C|GetCamera _output_get_2)))
  (bind _output_get_4 (Variables|Default|SetAngle (Math|Random|RandomFloatinRange 0.0 3.6e+02)))
  (bind _output_get_5 (Variables|Default|SetSpawnedCamLocation (Math|Vector|MakeVector (+ (.x (Transformation|GetWorldLocation (Variables|/Game/Core/ActorsAndControllers/ImpulsePlayer1_BP.ImpulsePlayer1_BP_C|GetCamera _output_get_2))) (* (Math|Trig|Cos(Degrees) _output_get_4) (Variables|Default|GetCircleRad))) (+ (.y (Transformation|GetWorldLocation (Variables|/Game/Core/ActorsAndControllers/ImpulsePlayer1_BP.ImpulsePlayer1_BP_C|GetCamera _output_get_2))) (* (Math|Trig|Sin(Degrees) _output_get_4) (Variables|Default|GetCircleRad))) (+ (.z (Transformation|GetWorldLocation (Variables|/Game/Core/ActorsAndControllers/ImpulsePlayer1_BP.ImpulsePlayer1_BP_C|GetCamera _output_get_2))) (Variables|Default|GetDistanceToGoAbove)))))
  (bind _returnvalue_2 (Game|SpawnActorfromClass "/Game/Core/ActorsAndControllers/CircleInPawn.CircleInPawn_C" (Math|Transform|MakeTransform _output_get_5 (Math|Rotator|FindLookatRotation _output_get_5 (Variables|Default|GetLookatLocation)) "1,1,1") "Undefined" 0 0))
  (Pawn|Possess (Variables|Default|GetPlayerController) _returnvalue_2)
  (Variables|Default|SetPlayerCamPawn _returnvalue_2))