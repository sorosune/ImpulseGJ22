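; Player actor that propels a physics sphere using a child die actor's six face arrows, driven by input actions 1 to 6.
; Each input applies an impulse opposite the chosen arrow's forward vector, scaled by ImpulseFactor.
; It also sets the die's spin from an axis-angle rotator between actor up and Arrow1, regardless of chosen face.
; Tick damps that rotation rate using RotationFriction.
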(event Custom|DieImpulse
  (params (Arrow :type Arrow%20Component%20Object%20Reference))
  (Physics|AddImpulse (Variables|Components|GetSphere) (* (* (Math|Vector|GetForwardVector Arrow) -1.0) (Variables|Default|GetImpulse%20Factor)) "None" false))

(event EventBeginPlay
  (bind _asdice_bp (Utilities|Casting|CastToDice_BP (Variables|/Script/Engine.ChildActorComponent|GetChildActor (Variables|Components|GetDie))))
  (Variables|Default|SetAs%20Dice%20BP _asdice_bp))

(event Collision|EventActorBeginOverlap
  (params (OtherActor :type Actor%20Object%20Reference)))

(event EventTick
  (params (DeltaSeconds :type Float%20%28single-precision%29))
  ;[1 1 1] Slow Rotation
  (Variables|/Script/Engine.RotatingMovementComponent|SetRotationRate (Variables|/Game/Core/ActorsAndControllers/Dice_BP.Dice_BP_C|GetRotatingMovement (Variables|Default|GetAs%20Dice%20BP)) (* (Variables|/Script/Engine.RotatingMovementComponent|GetRotationRate (Variables|/Game/Core/ActorsAndControllers/Dice_BP.Dice_BP_C|GetRotatingMovement (Variables|Default|GetAs%20Dice%20BP))) (- 1.0 (* DeltaSeconds (Variables|Default|GetRotationFriction))))))

(event Input|ActionEvents|InputAction1
  (params (Key :type Key%20Structure :default "None"))
  (bind _as_dice_bp (Variables|Default|GetAs%20Dice%20BP))
  (bind _arrow1 (Variables|/Game/Core/ActorsAndControllers/Dice_BP.Dice_BP_C|GetArrow1 _as_dice_bp))
  (:Pressed
    (Variables|Default|SetDiceFace 1)
    (CallFunction|DieImpulse (Utilities|Select :Index (Variables|Default|GetDiceFace) :Option%200 0 :Option%201 _arrow1 :Option%202 (Variables|/Game/Core/ActorsAndControllers/Dice_BP.Dice_BP_C|GetArrow2 _as_dice_bp) :Option%203 (Variables|/Game/Core/ActorsAndControllers/Dice_BP.Dice_BP_C|GetArrow3 _as_dice_bp) :Option%204 (Variables|/Game/Core/ActorsAndControllers/Dice_BP.Dice_BP_C|GetArrow4 _as_dice_bp) :Option%205 (Variables|/Game/Core/ActorsAndControllers/Dice_BP.Dice_BP_C|GetArrow5 _as_dice_bp) :Option%206 (Variables|/Game/Core/ActorsAndControllers/Dice_BP.Dice_BP_C|GetArrow6 _as_dice_bp)))
    (bind _rotator (CallFunction|GetRotatorforDie _arrow1))
    (Variables|/Script/Engine.RotatingMovementComponent|SetRotationRate (Variables|/Game/Core/ActorsAndControllers/Dice_BP.Dice_BP_C|GetRotatingMovement (Variables|Default|GetAs%20Dice%20BP)) _rotator)))

(event Input|ActionEvents|InputAction2
  (params (Key :type Key%20Structure :default "None"))
  (bind _as_dice_bp (Variables|Default|GetAs%20Dice%20BP))
  (bind _arrow1 (Variables|/Game/Core/ActorsAndControllers/Dice_BP.Dice_BP_C|GetArrow1 _as_dice_bp))
  (:Pressed
    (Variables|Default|SetDiceFace 2)
    (CallFunction|DieImpulse (Utilities|Select :Index (Variables|Default|GetDiceFace) :Option%200 0 :Option%201 _arrow1 :Option%202 (Variables|/Game/Core/ActorsAndControllers/Dice_BP.Dice_BP_C|GetArrow2 _as_dice_bp) :Option%203 (Variables|/Game/Core/ActorsAndControllers/Dice_BP.Dice_BP_C|GetArrow3 _as_dice_bp) :Option%204 (Variables|/Game/Core/ActorsAndControllers/Dice_BP.Dice_BP_C|GetArrow4 _as_dice_bp) :Option%205 (Variables|/Game/Core/ActorsAndControllers/Dice_BP.Dice_BP_C|GetArrow5 _as_dice_bp) :Option%206 (Variables|/Game/Core/ActorsAndControllers/Dice_BP.Dice_BP_C|GetArrow6 _as_dice_bp)))
    (bind _rotator (CallFunction|GetRotatorforDie _arrow1))
    (Variables|/Script/Engine.RotatingMovementComponent|SetRotationRate (Variables|/Game/Core/ActorsAndControllers/Dice_BP.Dice_BP_C|GetRotatingMovement (Variables|Default|GetAs%20Dice%20BP)) _rotator)))

(event Input|ActionEvents|InputAction3
  (params (Key :type Key%20Structure :default "None"))
  (bind _as_dice_bp (Variables|Default|GetAs%20Dice%20BP))
  (bind _arrow1 (Variables|/Game/Core/ActorsAndControllers/Dice_BP.Dice_BP_C|GetArrow1 _as_dice_bp))
  (:Pressed
    (Variables|Default|SetDiceFace 3)
    (CallFunction|DieImpulse (Utilities|Select :Index (Variables|Default|GetDiceFace) :Option%200 0 :Option%201 _arrow1 :Option%202 (Variables|/Game/Core/ActorsAndControllers/Dice_BP.Dice_BP_C|GetArrow2 _as_dice_bp) :Option%203 (Variables|/Game/Core/ActorsAndControllers/Dice_BP.Dice_BP_C|GetArrow3 _as_dice_bp) :Option%204 (Variables|/Game/Core/ActorsAndControllers/Dice_BP.Dice_BP_C|GetArrow4 _as_dice_bp) :Option%205 (Variables|/Game/Core/ActorsAndControllers/Dice_BP.Dice_BP_C|GetArrow5 _as_dice_bp) :Option%206 (Variables|/Game/Core/ActorsAndControllers/Dice_BP.Dice_BP_C|GetArrow6 _as_dice_bp)))
    (bind _rotator (CallFunction|GetRotatorforDie _arrow1))
    (Variables|/Script/Engine.RotatingMovementComponent|SetRotationRate (Variables|/Game/Core/ActorsAndControllers/Dice_BP.Dice_BP_C|GetRotatingMovement (Variables|Default|GetAs%20Dice%20BP)) _rotator)))

(event Input|ActionEvents|InputAction4
  (params (Key :type Key%20Structure :default "None"))
  (bind _as_dice_bp (Variables|Default|GetAs%20Dice%20BP))
  (bind _arrow1 (Variables|/Game/Core/ActorsAndControllers/Dice_BP.Dice_BP_C|GetArrow1 _as_dice_bp))
  (:Pressed
    (Variables|Default|SetDiceFace 4)
    (CallFunction|DieImpulse (Utilities|Select :Index (Variables|Default|GetDiceFace) :Option%200 0 :Option%201 _arrow1 :Option%202 (Variables|/Game/Core/ActorsAndControllers/Dice_BP.Dice_BP_C|GetArrow2 _as_dice_bp) :Option%203 (Variables|/Game/Core/ActorsAndControllers/Dice_BP.Dice_BP_C|GetArrow3 _as_dice_bp) :Option%204 (Variables|/Game/Core/ActorsAndControllers/Dice_BP.Dice_BP_C|GetArrow4 _as_dice_bp) :Option%205 (Variables|/Game/Core/ActorsAndControllers/Dice_BP.Dice_BP_C|GetArrow5 _as_dice_bp) :Option%206 (Variables|/Game/Core/ActorsAndControllers/Dice_BP.Dice_BP_C|GetArrow6 _as_dice_bp)))
    (bind _rotator (CallFunction|GetRotatorforDie _arrow1))
    (Variables|/Script/Engine.RotatingMovementComponent|SetRotationRate (Variables|/Game/Core/ActorsAndControllers/Dice_BP.Dice_BP_C|GetRotatingMovement (Variables|Default|GetAs%20Dice%20BP)) _rotator)))

(event Input|ActionEvents|InputAction5
  (params (Key :type Key%20Structure :default "None"))
  (bind _as_dice_bp (Variables|Default|GetAs%20Dice%20BP))
  (bind _arrow1 (Variables|/Game/Core/ActorsAndControllers/Dice_BP.Dice_BP_C|GetArrow1 _as_dice_bp))
  (:Pressed
    (Variables|Default|SetDiceFace 5)
    (CallFunction|DieImpulse (Utilities|Select :Index (Variables|Default|GetDiceFace) :Option%200 0 :Option%201 _arrow1 :Option%202 (Variables|/Game/Core/ActorsAndControllers/Dice_BP.Dice_BP_C|GetArrow2 _as_dice_bp) :Option%203 (Variables|/Game/Core/ActorsAndControllers/Dice_BP.Dice_BP_C|GetArrow3 _as_dice_bp) :Option%204 (Variables|/Game/Core/ActorsAndControllers/Dice_BP.Dice_BP_C|GetArrow4 _as_dice_bp) :Option%205 (Variables|/Game/Core/ActorsAndControllers/Dice_BP.Dice_BP_C|GetArrow5 _as_dice_bp) :Option%206 (Variables|/Game/Core/ActorsAndControllers/Dice_BP.Dice_BP_C|GetArrow6 _as_dice_bp)))
    (bind _rotator (CallFunction|GetRotatorforDie _arrow1))
    (Variables|/Script/Engine.RotatingMovementComponent|SetRotationRate (Variables|/Game/Core/ActorsAndControllers/Dice_BP.Dice_BP_C|GetRotatingMovement (Variables|Default|GetAs%20Dice%20BP)) _rotator)))

(event Input|ActionEvents|InputAction6
  (params (Key :type Key%20Structure :default "None"))
  (bind _as_dice_bp (Variables|Default|GetAs%20Dice%20BP))
  (bind _arrow1 (Variables|/Game/Core/ActorsAndControllers/Dice_BP.Dice_BP_C|GetArrow1 _as_dice_bp))
  (:Pressed
    (Variables|Default|SetDiceFace 6)
    (CallFunction|DieImpulse (Utilities|Select :Index (Variables|Default|GetDiceFace) :Option%200 0 :Option%201 _arrow1 :Option%202 (Variables|/Game/Core/ActorsAndControllers/Dice_BP.Dice_BP_C|GetArrow2 _as_dice_bp) :Option%203 (Variables|/Game/Core/ActorsAndControllers/Dice_BP.Dice_BP_C|GetArrow3 _as_dice_bp) :Option%204 (Variables|/Game/Core/ActorsAndControllers/Dice_BP.Dice_BP_C|GetArrow4 _as_dice_bp) :Option%205 (Variables|/Game/Core/ActorsAndControllers/Dice_BP.Dice_BP_C|GetArrow5 _as_dice_bp) :Option%206 (Variables|/Game/Core/ActorsAndControllers/Dice_BP.Dice_BP_C|GetArrow6 _as_dice_bp)))
    (bind _rotator (CallFunction|GetRotatorforDie _arrow1))
    (Variables|/Script/Engine.RotatingMovementComponent|SetRotationRate (Variables|/Game/Core/ActorsAndControllers/Dice_BP.Dice_BP_C|GetRotatingMovement (Variables|Default|GetAs%20Dice%20BP)) _rotator)))

(fn ConstructionScript)

(fn GetRotatorforDie
  (params (Arrow :type Arrow%20Component%20Object%20Reference))
  (bind _returnvalue (Math|Vector|GetForwardVector Arrow))
  (bind _returnvalue_2 (Transformation|GetActorUpVector))
  (return (Math|Vector|RotatorfromAxisandAngle (Math|Vector|Normalize (Math|Vector|CrossProduct _returnvalue_2 _returnvalue)) (Math|Trig|RadiansToDegrees (Math|Trig|Acos(Degrees) (Math|Vector|DotProduct _returnvalue_2 _returnvalue))))))