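; MainMenuImpulsePlayer_BP is the player actor for the main menu, handling the menu camera view.
; On BeginPlay it finds actors tagged "CameraLocation" and, if the first is valid, blends the first player controller's view target to it with an ease-out transition.
; Tick and overlap events are disabled stubs, and the construction script only calls its parent.
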(event EventBeginPlay
  (|CallParentFunction)
  (bind _outactors (Actor|GetAllActorswithTag "CameraLocation"))
  (Utilities|IsValid (Utilities|Array|Get(acopy) _outactors)
    (:Is%20Valid
      (Game|Player|SetViewTargetwithBlend (Game|GetPlayerController 0) (Utilities|Array|Get(acopy) _outactors) 2.0 "VTBlend_EaseOut" 2.0 false))))

(event Collision|EventActorBeginOverlap
  (params (OtherActor :type Actor%20Object%20Reference))
  (|CallParentFunction OtherActor) ; This node is disabled and will not be called.\nDrag off pins to build functionality.
)

(event EventTick
  (params (DeltaSeconds :type Float%20%28single-precision%29))
  (|CallParentFunction DeltaSeconds) ; This node is disabled and will not be called.\nDrag off pins to build functionality.
)

(fn ConstructionScript
  (|CallParentFunction))