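; Test player for dice-driven movement: six inputs fire impulses that push a physics sphere away from the matching arrow on a child die.
; Holding adds continuous thrust up to a time limit; release starts a cooldown and spins the die by impulse direction, slowed by friction each tick.
; Control rotation follows velocity until CameraTick is false, then view blends to a tagged camera.
; Also stores collected trophies in the game instance and updates the counter.
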(event Custom|End%20Held
  (CallFunction|OnDiceButtonReleased (Variables|Default|GetDiceFace)))

(event Custom|Reset%20Cooldown
  (Variables|Default|SetCooldown false))

(event Custom|CollectTrophy
  (params (Trophy :type Trophy%20BP%20Object%20Reference))
  (bind _asimpulse_game_instance_bp (Utilities|Casting|CastToImpulseGameInstance_BP (Game|GetGameInstance)))
  (bind _returnvalue (Utilities|Array|Add (Variables|/Game/Core/Systems/ImpulseGameInstance_BP.ImpulseGameInstance_BP_C|GetTrophies _asimpulse_game_instance_bp) Trophy))
  (Default|UpdateCount (Variables|Default|GetCollectibleCounter) (+ _returnvalue 1))
  (Actor|DestroyActor Trophy))

(event Custom|CamRotate
  (if (Variables|Default|GetbCameraTick)
    (bind _returnvalue (Physics|GetPhysicsLinearVelocity (Variables|Components|GetSphere) "None"))
    (Pawn|SetControlRotation (Game|GetPlayerController 0) (Math|Conversions|RotationFromXVector (Math|Vector|Normalize _returnvalue)))
    (else
      (Utilities|FlowControl|Sequence
        (:then_0
          (Utilities|FlowControl|DoOnce false
            (:Completed
              (Input|SetInputModeUIOnly (Game|GetPlayerController 0) 0 "LockInFullscreen")
              (Utilities|FlowControl|Delay 4.1)
              (bind _outactors (Actor|GetAllActorswithTag "CameraLocation"))
              (Utilities|IsValid (Utilities|Array|Get(acopy) _outactors)
                (:Is%20Valid
                  (Game|Player|SetViewTargetwithBlend (Game|GetPlayerController 0) (Utilities|Array|Get(acopy) _outactors) 2.0 "VTBlend_Cubic" 2.0 false))))))
        (:then_1
          (Utilities|FlowControl|DoOnce false
            (:Completed
              (Utilities|FlowControl|Delay 6.1)
              (Input|SetInputModeGameandUI (Game|GetPlayerController 0) 0 "DoNotLock" false))))))))

(event EventBeginPlay
  (bind _asdice_bp (Utilities|Casting|CastToDice_BP (Variables|/Script/Engine.ChildActorComponent|GetChildActor (Variables|Components|GetDie))))
  (Variables|Default|SetAs%20Dice%20BP _asdice_bp))

(event EventTick
  (params (DeltaSeconds :type Float%20%28single-precision%29))
  (CallFunction|TickRotation DeltaSeconds)
  (CallFunction|CamRotate)
  (if (Variables|Default|GetHeld)
    (Physics|AddImpulse (Variables|Components|GetSphere) (* (Variables|Default|GetImpulseDirection) (* DeltaSeconds (Variables|Default|GetImpulseHeld))) "None" true)))

(event Input|ActionEvents|InputAction1
  (params (Key :type Key%20Structure :default "None"))
  (:Pressed
    (Utilities|ButtonEventCall 1 :!label _label))
  (:Released
    (goto _label Button%20Up)))

(event Input|ActionEvents|InputAction2
  (params (Key :type Key%20Structure :default "None"))
  (:Pressed
    (Utilities|ButtonEventCall 2 :!label _label))
  (:Released
    (goto _label Button%20Up)))

(event Input|ActionEvents|InputAction3
  (params (Key :type Key%20Structure :default "None"))
  (:Pressed
    (Utilities|ButtonEventCall 3 :!label _label))
  (:Released
    (goto _label Button%20Up)))

(event Input|ActionEvents|InputAction4
  (params (Key :type Key%20Structure :default "None"))
  (:Pressed
    (Utilities|ButtonEventCall 4 :!label _label))
  (:Released
    (goto _label Button%20Up)))

(event Input|ActionEvents|InputAction5
  (params (Key :type Key%20Structure :default "None"))
  (:Pressed
    (Utilities|ButtonEventCall 5 :!label _label))
  (:Released
    (goto _label Button%20Up)))

(event Input|ActionEvents|InputAction6
  (params (Key :type Key%20Structure :default "None"))
  (:Pressed
    (Utilities|ButtonEventCall 6 :!label _label))
  (:Released
    (goto _label Button%20Up)))

(event Input|KeyboardEvents|F6
  (params (Key :type Key%20Structure :default "None")))

(event Input|KeyboardEvents|F7
  (params (Key :type Key%20Structure :default "None")))

(fn ConstructionScript)

(fn OnDiceButtonDown
  (params (Dice :type Integer))
  (bind _as_dice_bp (Variables|Default|GetAs%20Dice%20BP))
  (if (and (== (Variables|Default|GetDiceFace) 0) (not (Variables|Default|GetCooldown)))
    (Variables|Default|SetDiceFace Dice)
    (Variables|Default|SetImpulseDirection (* (Math|Vector|GetForwardVector (Utilities|Select :Index (Variables|Default|GetDiceFace) :Option%200 0 :Option%201 (Variables|/Game/Core/ActorsAndControllers/Dice_BP.Dice_BP_C|GetArrow1 _as_dice_bp) :Option%202 (Variables|/Game/Core/ActorsAndControllers/Dice_BP.Dice_BP_C|GetArrow2 _as_dice_bp) :Option%203 (Variables|/Game/Core/ActorsAndControllers/Dice_BP.Dice_BP_C|GetArrow3 _as_dice_bp) :Option%204 (Variables|/Game/Core/ActorsAndControllers/Dice_BP.Dice_BP_C|GetArrow4 _as_dice_bp) :Option%205 (Variables|/Game/Core/ActorsAndControllers/Dice_BP.Dice_BP_C|GetArrow5 _as_dice_bp) :Option%206 (Variables|/Game/Core/ActorsAndControllers/Dice_BP.Dice_BP_C|GetArrow6 _as_dice_bp))) -1.0))
    (Variables|Default|SetHeld true)
    (Utilities|Time|SetTimerbyFunctionName 0 "End Held" (Variables|Default|GetMaxHoldDuration))
    (Physics|AddImpulse (Variables|Components|GetSphere) (* (Variables|Default|GetImpulseDirection) (Variables|Default|GetImpulseFactor)) "None" true)
    (Variables|/Script/Engine.RotatingMovementComponent|SetRotationRate (Variables|/Game/Core/ActorsAndControllers/Dice_BP.Dice_BP_C|GetRotatingMovement (Variables|Default|GetAs%20Dice%20BP)) "0, 0, 0")))

(fn OnDiceButtonReleased
  (params (Dice :type Integer))
  (if (== Dice (Variables|Default|GetDiceFace))
    (Variables|Default|SetDiceFace 0)
    (Variables|Default|SetCooldown true)
    (Variables|Default|SetHeld false)
    (Utilities|Time|SetTimerbyFunctionName 0 "Reset Cooldown" (Variables|Default|GetCooldownTime))
    (Utilities|Time|ClearTimerbyFunctionName 0 "End Held")
    (bind _rotator (CallFunction|GetRotatorforDie))
    (Variables|/Script/Engine.RotatingMovementComponent|SetRotationRate (Variables|/Game/Core/ActorsAndControllers/Dice_BP.Dice_BP_C|GetRotatingMovement (Variables|Default|GetAs%20Dice%20BP)) (* _rotator (Variables|Default|GetRotationMultiplier)))))

(fn GetRotatorforDie
  (bind _returnvalue (Math|Trig|Atan2(Radians) 1.0 0.0))
  (bind _impulsedirection (Variables|Default|GetImpulseDirection))
  (bind _impulsedirection_2 (Variables|Default|GetImpulseDirection))
  (bind _returnvalue_2 (* _impulsedirection_2 -1.0))
  (bind (_x _y) (Math|Vector|BreakVector _impulsedirection))
  (bind _returnvalue_3 (Math|Vector|MakeVector _x _y 0.0))
  (bind _returnvalue_4 (Math|Vector|DotProduct _returnvalue_2 "0, 0,1.000000"))
  (bind _returnvalue_5 (Math|Vector|Normalize _returnvalue_3))
  (bind _returnvalue_6 (Math|Trig|Acos(Degrees) _returnvalue_4))
  (bind _returnvalue_7 (Math|Trig|Atan2(Radians) (.y _returnvalue_5) (.x _returnvalue_5)))
  (bind _returnvalue_8 (- _returnvalue_7 _returnvalue))
  (bind _returnvalue_9 (Math|Trig|RadiansToDegrees _returnvalue_8))
  (return (Math|Rotator|MakeRotator (Math|Trig|RadiansToDegrees (* _returnvalue_6 (Math|Trig|Cos(Degrees) _returnvalue_9))) (Math|Trig|RadiansToDegrees (* _returnvalue_6 (Math|Trig|Sin(Degrees) _returnvalue_9))) 0.0)))

(fn TickRotation
  (params (Delta%20Time :type Float%20%28single-precision%29))
  (Variables|/Script/Engine.RotatingMovementComponent|SetRotationRate (Variables|/Game/Core/ActorsAndControllers/Dice_BP.Dice_BP_C|GetRotatingMovement (Variables|Default|GetAs%20Dice%20BP)) (* (Variables|/Script/Engine.RotatingMovementComponent|GetRotationRate (Variables|/Game/Core/ActorsAndControllers/Dice_BP.Dice_BP_C|GetRotatingMovement (Variables|Default|GetAs%20Dice%20BP))) (- 1.0 (* Delta%20Time (Variables|Default|GetRotationFriction))))))

(fn RotateCamera)