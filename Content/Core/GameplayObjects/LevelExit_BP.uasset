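; Level exit trigger that records the level's completion time and sends the player to the next level.
; Tick accumulates elapsed time in whole milliseconds through a math expression node.
; When ImpulseGJ22Player overlaps the Collider, it passes the current level name and time as BestTime to the Impulse game instance, with no comparison here.
; It then saves the game and opens the next level by name.
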(event OnComponentBeginOverlap(Collider)
  (params (OverlappedComponent :type Primitive%20Component%20Object%20Reference) (OtherActor :type Actor%20Object%20Reference) (OtherComp :type Primitive%20Component%20Object%20Reference) (OtherBodyIndex :type Integer) (bFromSweep :type Boolean) (SweepResult :type Hit%20Result%20Structure%20%28by%20ref%29))
  (Utilities|Casting|CastToImpulseGJ22Player OtherActor)
  (bind _returnvalue (Class|ImpulseGameInstance|GetImpulseGameInstance))
  (Class|ImpulseGameInstance|SetLevelData _returnvalue (Utilities|Struct|MakeLevelData (Variables|Default|GetCurrentLevelName) (Variables|Default|GetCompletionTime)))
  (Class|ImpulseGameInstance|SaveGame _returnvalue)
  (Game|OpenLevel(byName) (Utilities|String|StringToName (Variables|Default|GetNextLevelName))))

(event EventBeginPlay)

(event Collision|EventActorBeginOverlap
  (params (OtherActor :type Actor%20Object%20Reference)))

(event EventTick
  (params (DeltaSeconds :type Float%20%28single-precision%29))
  (Variables|Default|SetCompletionTime (Math|Float|Truncate (|({A703CB62-423A-F555-7BF3-50857519A7F4}+(DeltaSeconds*1000)) DeltaSeconds))))

(fn ConstructionScript)